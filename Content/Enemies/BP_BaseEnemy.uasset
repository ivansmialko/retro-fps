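; Base enemy character drawn as directional Paper2D flipbooks in a 3D world, with health, melee and ranged attacks.
; Each tick it picks a sprite from the player's angle and the idle, moving or attack state.
; Pawn sensing drives turning toward the player and a Blackboard sight flag that clears after a short delay.
; Death stops AI and collision, plays hardcoded flamethrower death flipbooks, then destroys the actor.
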(event `self.ReceiveTick`
  (params (DeltaSeconds :type "Float (single-precision)"))
  (bind _returnvalue (`KismetMathLibrary.Normal` (- (`self.K2_GetActorLocation` (`GameplayStatics.GetPlayerCharacter` 0)) (`self.K2_GetActorLocation`))))
  (if (`self.IsDead?`)
    (`self.HandleDeath`)
    (else
      (`self.UpdateAnimationState`)
      (if (`self.CanSeePlayer?`)
        (`self.RotateTowardsPlayer`))
      (set `self.Degrees` (`KismetMathLibrary.DegAcos` (`KismetMathLibrary.Dot_VectorVector` (`self.GetActorForwardVector`) _returnvalue)))
      (if (< (`KismetMathLibrary.Dot_VectorVector` (`self.GetActorRightVector`) _returnvalue) 0.0)
        ;[1 1 1] Player is on the right side from enemy
        (`/Engine/EditorBlueprintResources/StandardMacros.CompareFloat` (`self.Degrees`) 180.0
          (:`>`
            (`self.SetFlipbook` (struct :`Yaw` -90.0) 0 "front" :!label _label))
          (:`==`
            (goto _label))
          (:`<`
            (`/Engine/EditorBlueprintResources/StandardMacros.CompareFloat` (`self.Degrees`) 135.0
              (:`>`
                (`self.SetFlipbook` (struct :`Yaw` 135.0) 3 "back left" :!label _label_2))
              (:`==`
                (goto _label_2))
              (:`<`
                (`/Engine/EditorBlueprintResources/StandardMacros.CompareFloat` (`self.Degrees`) 90.0
                  (:`>`
                    (`self.SetFlipbook` (struct :`Yaw` 180.0) 2 "left" :!label _label_3))
                  (:`==`
                    (goto _label_3))
                  (:`<`
                    (`/Engine/EditorBlueprintResources/StandardMacros.CompareFloat` (`self.Degrees`) 45.0
                      (:`>`
                        (`self.SetFlipbook` (struct :`Yaw` 45.0) 1 "front right" :!label _label_4))
                      (:`==`
                        (goto _label_4))
                      (:`<`
                        (`self.SetFlipbook` (struct :`Yaw` -90.0) 0 "front")))))))))
        (else
          ;[1 1 1] Player is on the left side from enemy
          (`/Engine/EditorBlueprintResources/StandardMacros.CompareFloat` (`self.Degrees`) 180.0
            (:`>`
              (`self.SetFlipbook` (struct :`Yaw` -45.0) 7 "front left" :!label _label_5))
            (:`==`
              (goto _label_5))
            (:`<`
              (`/Engine/EditorBlueprintResources/StandardMacros.CompareFloat` (`self.Degrees`) 135.0
                (:`>`
                  (`self.SetFlipbook` (struct :`Yaw` 90.0) 4 "back" :!label _label_6))
                (:`==`
                  (goto _label_6))
                (:`<`
                  (`/Engine/EditorBlueprintResources/StandardMacros.CompareFloat` (`self.Degrees`) 90.0
                    (:`>`
                      (`self.SetFlipbook` (struct :`Yaw` 45.0) 5 "back right" :!label _label_7))
                    (:`==`
                      (goto _label_7))
                    (:`<`
                      (`/Engine/EditorBlueprintResources/StandardMacros.CompareFloat` (`self.Degrees`) 45.0
                        (:`>`
                          (`self.SetFlipbook` (struct) 6 "right" :!label _label_8))
                        (:`==`
                          (goto _label_8))
                        (:`<`
                          (`self.SetFlipbook` (struct :`Yaw` -45.0) 1 "front left"))))))))))))))

(event `HandleDeath`
  (bind (_returnvalue_roll _returnvalue_pitch _returnvalue_yaw) (`KismetMathLibrary.BreakRotator` (`KismetMathLibrary.FindLookAtRotation` (`self.K2_GetActorLocation`) (`self.K2_GetActorLocation` (`GameplayStatics.GetPlayerCharacter` 0)))))
  (`self.K2_SetActorRotation` (`KismetMathLibrary.MakeRotator` 0.0 0.0 _returnvalue_yaw))
  (`/Engine/EditorBlueprintResources/StandardMacros.DoOnce` false
    (:`Completed`
      (`BrainComponent.StopLogic` (`AIController.BrainComponent` (`AIBlueprintHelperLibrary.GetAIController` self)) "Is dead")
      (`CharacterMovementComponent.SetMovementMode` (`self.CharacterMovement`) "MOVE_Flying" 0)
      (`ActorComponent.Deactivate` (`self.CharacterMovement`))
      (`PrimitiveComponent.SetCollisionEnabled` (`self.CapsuleComponent`) "NoCollision")
      (`SceneComponent.K2_SetRelativeRotation` (`self.PaperFlipbook`) (struct :`Yaw` -90.0) false false)
      (`PaperFlipbookComponent.SetFlipbook` (`self.PaperFlipbook`) "/Game/Sprites/Enemy/Firedemon/Death/PFB_Flamethrower_Death.PFB_Flamethrower_Death")
      (`KismetSystemLibrary.Delay` (- (`PaperFlipbookComponent.GetFlipbookLength` (`self.PaperFlipbook`)) 0.2))
      (`PaperFlipbookComponent.SetFlipbook` (`self.PaperFlipbook`) "/Game/Sprites/Enemy/Firedemon/Death/PFB_Flamethrower_Dead.PFB_Flamethrower_Dead")
      (`self.K2_AddActorLocalOffset` (0.0 0.0 -50.0))
      (`KismetSystemLibrary.Delay` 5.0)
      (`self.K2_DestroyActor`))))

(event `self.ReceiveBeginPlay`
  ;[0 0.957 1 0.5] Initialization
  (set `self.Health` (`self.BaseHealth`))
  (set `CharacterMovementComponent.MaxWalkSpeed` (`self.BaseSpeed`) (`self.CharacterMovement`)))

(event `self.ReceiveAnyDamage`
  (params (Damage :type "Float (single-precision)") (DamageType :type "DamageType Object Reference") (InstigatedBy :type "Controller Object Reference") (DamageCauser :type "Actor Object Reference"))
  (bind _output_get (set `self.Health` (- (`self.Health`) Damage)))
  (if (<= _output_get 0.0)
    (set `self.IsDead?` true)
    (`KismetSystemLibrary.PrintString` "бля пизда")))

(event `RotateTowardsPlayer`
  ;[0.9588 0.02083 1 0.5] Rotate to player
  (`self.K2_SetActorRotation` (`KismetMathLibrary.RInterpTo` (`self.K2_GetActorRotation`) (`KismetMathLibrary.FindLookAtRotation` (`self.K2_GetActorLocation`) (`self.K2_GetActorLocation` (`GameplayStatics.GetPlayerCharacter` 0))) (`GameplayStatics.GetWorldDeltaSeconds`) (`self.RotationSpeed`))))

(event `self.PawnSensing.OnSeePawn`
  (params (Pawn :type "Pawn Object Reference"))
  ;[0.1164 1 0 0.5] Player detection
  (cast `/Game/FirstPerson/Blueprints/BP_FirstPersonCharacter` Pawn)
  (bind _output_get (set `self.CanSeePlayer?` true))
  (`BlackboardComponent.SetValueAsBool` (`AIBlueprintHelperLibrary.GetBlackboard` null) "CanSeePlayer" _output_get)
  (`KismetSystemLibrary.RetriggerableDelay` 0.7)
  (bind _output_get_2 (set `self.CanSeePlayer?` false))
  (`BlackboardComponent.SetValueAsBool` (`AIBlueprintHelperLibrary.GetBlackboard` null) "CanSeePlayer" _output_get_2))

(event `SpawnProjectile`
  ;[1 0 0 0.5] Ranged attack
  (set `self.AttackState` "NewEnumerator1")
  (`MovementComponent.StopMovementImmediately` (`self.CharacterMovement`))
  (`|SpawnActorFromClass` "/Game/Blueprints/Projectiles/BP_EnemyProjectile.BP_EnemyProjectile_C" (`SceneComponent.K2_GetComponentToWorld` (`self.ProjectileSpawn`)) "Undefined" "OverrideRootScale" null (`self.Projectile Speed`) (`self.Projectile Damage`) null)
  (`KismetSystemLibrary.RetriggerableDelay` (+ (`self.RangedRate`) 0.1))
  (set `self.AttackState` "NewEnumerator2"))

(event `MeleeAttack`
  ;[1 0.9624 0 0.5] Melee attack
  (bind _returnvalue (`self.IsEnemyCanHitPlayer`))
  (if _returnvalue
    (set `self.AttackState` "NewEnumerator0")
    (`GameplayStatics.ApplyDamage` (`GameplayStatics.GetPlayerCharacter` 0) (`self.Melee Damage`))
    (`KismetSystemLibrary.RetriggerableDelay` (+ (`self.MeleeRate`) 0.1))
    (set `self.AttackState` "NewEnumerator2")))

(fn `IsEnemyAtMovement`
  (returns (ReturnValue :type Boolean))
  (return (> (`KismetMathLibrary.VSize` (`MovementComponent.Velocity` (`self.CharacterMovement`))) 0.0)))

(fn `IsEnemyCanHitPlayer`
  (returns (ReturnValue :type Boolean))
  (bind _returnvalue (`self.K2_GetActorLocation`))
  (bind _outhit (`KismetSystemLibrary.LineTraceSingleForObjects` _returnvalue (+ _returnvalue (* (`self.GetActorForwardVector`) 200.0)) (`|MakeArray` "ObjectTypeQuery3" :!type "EObjectTypeQuery Enum") false (`|MakeArray` self :!type "Actor Object Reference") "ForDuration"))
  (return (== (`.HitActor` (`GameplayStatics.BreakHitResult` _outhit)) (`GameplayStatics.GetPlayerCharacter` 0))))

(fn `SetFlipbook`
  (params (TargetRotation :type "Rotator Structure") (TargetSpriteId :type Integer) (LogString :type String))
  (locals (LocalTargetLocation :type "Rotator Structure") (LocalTargetSpriteId :type Integer) (LocalLogString :type String) (LocalTargetFlipbookArray :type "Array of PaperFlipbook Object Reference"))
  (set `local.LocalTargetLocation` TargetRotation)
  (set `local.LocalTargetSpriteId` TargetSpriteId)
  (set `local.LocalLogString` LogString)
  (set `local.LocalTargetFlipbookArray` (select `/Game/Enemies/EnemyAnimationState` (`self.EnemyAnimationState`) :`NewEnumerator0` (`self.FlipBooksIdle`) :`NewEnumerator1` (`self.FlipBooksMoving`) :`NewEnumerator2` (`self.FlipBooksAttackMelee`) :`NewEnumerator3` (`self.FlipBooksAttackRanged`)))
  (`SceneComponent.K2_SetRelativeRotation` (`self.PaperFlipbook`) (`local.LocalTargetLocation`) false false)
  (`PaperFlipbookComponent.SetFlipbook` (`self.PaperFlipbook`) (`|GetArrayItem` (`local.LocalTargetFlipbookArray`) (`local.LocalTargetSpriteId`))))

(fn `UpdateAnimationState`
  (switch `/Game/Enemies/EnemyAttackingState` (`self.AttackState`)
    (:`NewEnumerator2`
      (if (`self.IsEnemyAtMovement`)
        (set `self.EnemyAnimationState` "NewEnumerator1")
        (else
          (set `self.EnemyAnimationState` "NewEnumerator0"))))
    (:`NewEnumerator0`
      (set `self.EnemyAnimationState` (select `/Game/Enemies/EnemyAttackingState` (`self.AttackState`) :`NewEnumerator2` "NewEnumerator0" :`NewEnumerator0` "NewEnumerator2" :`NewEnumerator1` "NewEnumerator3" :!type "/Game/Enemies/EnemyAnimationState Enum") :!label _label))
    (:`NewEnumerator1`
      (goto _label))))

(fn `UserConstructionScript`)