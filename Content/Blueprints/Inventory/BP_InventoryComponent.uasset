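; Inventory component that stores the key cards held by its owner in a KeyCards collection.
; AddKeyCard and RemoveKeyCard both gate their change on IsHaveKeyCard, which returns true when the type is not found, despite its name.
; Adding therefore skips duplicates, while removal only runs for absent cards and never removes a held one.
; BeginPlay and Tick are unused.
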(fn `AddKeyCard`
  (params (KeyCardType :type "/Game/Blueprints/Items/KeyCard Enum" :default "NewEnumerator0"))
  (locals (Local_KeyCardType :type "/Game/Blueprints/Items/KeyCard Enum" :default "NewEnumerator0"))
  (bind _output_get (set `local.Local_KeyCardType` KeyCardType))
  (if (`self.IsHaveKeyCard` _output_get)
    (`KismetArrayLibrary.Array_Add` (`self.KeyCards`) (`local.Local_KeyCardType`))))

(fn `IsHaveKeyCard`
  (params (KeyCardType :type "/Game/Blueprints/Items/KeyCard Enum" :default "NewEnumerator0"))
  (returns (HaveKeyCard :type Boolean))
  (return (== (`KismetArrayLibrary.Array_Find` (`self.KeyCards`) KeyCardType) -1)))

(fn `RemoveKeyCard`
  (params (KeyCardType :type "/Game/Blueprints/Items/KeyCard Enum" :default "NewEnumerator0"))
  (locals (Local_KeyCardType :type "/Game/Blueprints/Items/KeyCard Enum" :default "NewEnumerator0"))
  (bind _output_get (set `local.Local_KeyCardType` KeyCardType))
  (if (`self.IsHaveKeyCard` _output_get)
    (`KismetArrayLibrary.Array_RemoveItem` (`self.KeyCards`) (`local.Local_KeyCardType`))))