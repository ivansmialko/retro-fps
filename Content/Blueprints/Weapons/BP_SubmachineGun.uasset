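; Submachine gun weapon Blueprint that fires automatically from the start of shooting until it is stopped.
; StartShooting passes a DoOnce gate to start a fast looping timer that checks ammo, decrements it, fires and shows the firing flipbook.
; Without ammo the timer keeps running but shows the idle flipbook.
; StopShooting clears the timer, restores the idle flipbook and resets the gate.
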(event `self.StartShooting`
  (`/Engine/EditorBlueprintResources/StandardMacros.DoOnce` false :!label _label
    (:`Completed`
      (bind _returnvalue (`KismetSystemLibrary.K2_SetTimerDelegate` (delegate `FireSubmachineGun`) 0.01 true))
      (set `self.SubmachineGunEvent` _returnvalue))))

(event `ResetFire`
  (goto _label :!via `Reset`))

(event `FireSubmachineGun`
  (bind _hasammo (`self.HasEnoughAmmo?`))
  (if _hasammo
    (`self.DecreaseAmmoAmount`)
    (`self.FireWeapon`)
    (`PaperFlipbookComponent.SetFlipbook` (`self.WeaponFlipbook`) "/Game/Sprites/Weapons/MiniGun/Sprites/PFB_SubmachineFire.PFB_SubmachineFire")
    (else
      (`PaperFlipbookComponent.SetFlipbook` (`self.WeaponFlipbook`) "/Game/Sprites/Weapons/MiniGun/Sprites/PFB_SubmachineGun_Idle.PFB_SubmachineGun_Idle"))))

(event `self.StopShooting`
  (`KismetSystemLibrary.K2_ClearAndInvalidateTimerHandle` (`self.SubmachineGunEvent`))
  (`PaperFlipbookComponent.SetFlipbook` (`self.WeaponFlipbook`) "/Game/Sprites/Weapons/MiniGun/Sprites/PFB_SubmachineGun_Idle.PFB_SubmachineGun_Idle")
  (`self.ResetFire`))

(fn `UserConstructionScript`
  (`parent.UserConstructionScript`))