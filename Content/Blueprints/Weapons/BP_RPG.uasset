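; BP_RPG is a rocket launcher weapon Blueprint that fires a projectile when shooting starts and ammo is available.
; A DoOnce gate blocks repeat fire while it triggers OnShoot and FireProjectile, then plays the fire flipbook.
; After a delay equal to that flipbook's length, it restores the idle flipbook and calls ResetWeapon to reopen the gate.
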(event `self.ReceiveBeginPlay`
  (`parent.ReceiveBeginPlay`)
  (`self.HasEnoughAmmo?`))

(event `self.StartShooting`
  (bind _weaponflipbook (`self.WeaponFlipbook`))
  (bind _hasammo (`self.HasEnoughAmmo?`))
  (if _hasammo
    (`/Engine/EditorBlueprintResources/StandardMacros.DoOnce` false :!label _label
      (:`Completed`
        (`self.OnShoot`)
        (`self.FireProjectile`)
        (`PaperFlipbookComponent.SetFlipbook` _weaponflipbook "/Game/Sprites/Weapons/RPG/Sprites/PFB_RPG_Fire.PFB_RPG_Fire")
        (`KismetSystemLibrary.Delay` (`PaperFlipbookComponent.GetFlipbookLength` _weaponflipbook))
        (`PaperFlipbookComponent.SetFlipbook` (`self.WeaponFlipbook`) "/Game/Sprites/Weapons/RPG/Sprites/RPG_Idle.RPG_Idle")
        (`self.ResetWeapon`)))))

(event `ResetWeapon`
  (goto _label :!via `Reset`))

(fn `UserConstructionScript`
  (`parent.UserConstructionScript`))