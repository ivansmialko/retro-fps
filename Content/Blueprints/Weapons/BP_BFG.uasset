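; BFG weapon Blueprint that fires a projectile when the player's cell ammo exceeds the required amount.
; StartShooting passes a DoOnce gate, sets the fire flipbook and waits for its length before calling FireProjectile, so the shot follows the animation.
; It then calls DecreaseShellAmount, despite checking cells, and ResetWeapon reopens the gate for the next shot.
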(event `self.StartShooting`
  (if (> (`/Game/FirstPerson/Blueprints/BP_FirstPersonCharacter.CellAmount` (`self.PlayerCharacterRef`)) (`self.NeedAmmoToFire`))
    (`/Engine/EditorBlueprintResources/StandardMacros.DoOnce` false :!label _label
      (:`Completed`
        (`PaperFlipbookComponent.SetFlipbook` (`self.WeaponFlipbook`) "/Game/Sprites/Weapons/BFG/Sprites/PFB_BFG_Fire.PFB_BFG_Fire")
        (`KismetSystemLibrary.Delay` (`PaperFlipbookComponent.GetFlipbookLength` (`self.WeaponFlipbook`)))
        (`self.FireProjectile`)
        (`self.DecreaseShellAmount`)
        (`self.ResetWeapon`)))))

(event `ResetWeapon`
  (goto _label :!via `Reset`))

(fn `UserConstructionScript`
  (`parent.UserConstructionScript`))