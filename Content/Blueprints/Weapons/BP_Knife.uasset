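; BP_Knife is a knife weapon Blueprint that plays a flipbook attack animation when used.
; StartShooting passes through a DoOnce gate, calls FireWeapon and switches the weapon flipbook from idle to attack.
; After a delay equal to the attack flipbook's length, it restores the idle flipbook and calls ResetWeapon to reopen the gate, so attacks cannot overlap.
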(event `self.StartShooting`
  (`/Engine/EditorBlueprintResources/StandardMacros.DoOnce` false :!label _label
    (:`Completed`
      (`self.FireWeapon`)
      (`PaperFlipbookComponent.SetFlipbook` (`self.WeaponFlipbook`) "/Game/Sprites/Weapons/Knife/Sprite/PFB_Knife_Attack.PFB_Knife_Attack")
      (`KismetSystemLibrary.Delay` (`PaperFlipbookComponent.GetFlipbookLength` (`self.WeaponFlipbook`)))
      (`PaperFlipbookComponent.SetFlipbook` (`self.WeaponFlipbook`) "/Game/Sprites/Weapons/Knife/Sprite/PFB_Knife_Idle.PFB_Knife_Idle")
      (`self.ResetWeapon`))))

(event `ResetWeapon`
  (goto _label :!via `Reset`))

(fn `UserConstructionScript`
  (`parent.UserConstructionScript`))