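; Plasma gun weapon Blueprint that fires automatically, submachine-gun style, between start and stop shooting events.
; StartShooting passes a DoOnce gate to start a fast looping timer that calls FireSubmachineGun.
; Each tick of that timer checks ammo, then either spends it, fires a projectile and shows the firing flipbook, or shows the idle one.
; StopShooting clears the timer, restores the idle flipbook and resets the gate.
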(event `self.StartShooting`
  (`/Engine/EditorBlueprintResources/StandardMacros.DoOnce` false :!label _label
    (:`Completed`
      (bind _returnvalue (`KismetSystemLibrary.K2_SetTimerDelegate` (delegate `FireSubmachineGun`) 0.05 true))
      (set `self.SubmachineGunEvent` _returnvalue))))

(event `ResetFire`
  (goto _label :!via `Reset`))

(event `FireSubmachineGun`
  (bind _hasammo (`self.HasEnoughAmmo?`))
  (if _hasammo
    (`self.DecreaseAmmoAmount`)
    (`self.FireProjectile`)
    (`PaperFlipbookComponent.SetFlipbook` (`self.WeaponFlipbook`) "/Game/Sprites/Weapons/PlasmaGun/Sprites/PFB_PlasmaGun_Fire.PFB_PlasmaGun_Fire")
    (else
      (`PaperFlipbookComponent.SetFlipbook` (`self.WeaponFlipbook`) "/Game/Sprites/Weapons/PlasmaGun/Sprites/PFB_PlasmaGun_Idle.PFB_PlasmaGun_Idle"))))

(event `self.StopShooting`
  (`KismetSystemLibrary.K2_ClearAndInvalidateTimerHandle` (`self.SubmachineGunEvent`))
  (`PaperFlipbookComponent.SetFlipbook` (`self.WeaponFlipbook`) "/Game/Sprites/Weapons/PlasmaGun/Sprites/PFB_PlasmaGun_Idle.PFB_PlasmaGun_Idle")
  (`self.ResetFire`))

(fn `UserConstructionScript`
  (`parent.UserConstructionScript`))