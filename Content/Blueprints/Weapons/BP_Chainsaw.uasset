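; BP_Chainsaw is a chainsaw weapon that fires after a short wind-up and shows its state through flipbook animation.
; StartShooting passes a DoOnce gate to set a brief non-looping timer for UseChainsaw, which calls FireWeapon and switches to the fire flipbook.
; StopShooting clears that timer, restores the idle flipbook and re-arms the gate via ResetWeapon, so releasing early cancels the pending attack.
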(event `self.StartShooting`
  (`/Engine/EditorBlueprintResources/StandardMacros.DoOnce` false :!label _label
    (:`Completed`
      (bind _returnvalue (`KismetSystemLibrary.K2_SetTimerDelegate` (delegate `UseChainsaw`) 0.15))
      (set `self.ChainsawEventRef` _returnvalue))))

(event `ResetWeapon`
  (goto _label :!via `Reset`))

(event `UseChainsaw`
  (`self.FireWeapon`)
  (`PaperFlipbookComponent.SetFlipbook` (`self.WeaponFlipbook`) "/Game/Sprites/Weapons/Chainsaw/Sprites/PFB_Chainsaw_Fire.PFB_Chainsaw_Fire"))

(event `self.StopShooting`
  (`KismetSystemLibrary.K2_ClearAndInvalidateTimerHandle` (`self.ChainsawEventRef`))
  (`PaperFlipbookComponent.SetFlipbook` (`self.WeaponFlipbook`) "/Game/Sprites/Weapons/Chainsaw/Sprites/PFB_Chainsaw_Idle.PFB_Chainsaw_Idle")
  (`self.ResetWeapon`))

(fn `UserConstructionScript`
  (`parent.UserConstructionScript`))