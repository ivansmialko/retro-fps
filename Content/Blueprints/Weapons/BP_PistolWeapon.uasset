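; Pistol weapon Blueprint that fires a shot and plays its Paper2D flipbook animation when StartShooting is triggered.
; A DoOnce gate calls FireWeapon, switches WeaponFlipbook to the fire animation, waits for its length, then restores the idle flipbook.
; ResetWeapon then reopens the gate, so the fire animation's length sets the minimum interval between shots.
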(event `self.StartShooting`
  (bind _weaponflipbook (`self.WeaponFlipbook`))
  (`/Engine/EditorBlueprintResources/StandardMacros.DoOnce` false :!label _label
    (:`Completed`
      (`self.FireWeapon`)
      (`PaperFlipbookComponent.SetFlipbook` _weaponflipbook "/Game/Sprites/Weapons/Pistol/Sprites/PFB_PistolFire.PFB_PistolFire")
      (`KismetSystemLibrary.Delay` (`PaperFlipbookComponent.GetFlipbookLength` _weaponflipbook))
      (`PaperFlipbookComponent.SetFlipbook` (`self.WeaponFlipbook`) "/Game/Sprites/Weapons/Pistol/Sprites/PFB_PistolIde.PFB_PistolIde")
      (`self.ResetWeapon`))))

(event `ResetWeapon`
  (goto _label :!via `Reset`))

(fn `UserConstructionScript`
  (`parent.UserConstructionScript`))