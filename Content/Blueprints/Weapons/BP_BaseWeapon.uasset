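; Base weapon actor for the first-person character, providing shared firing and ammo logic with empty start/stop shooting and description events.
; FireWeapon line-traces forward, damages the hit actor and spawns blood on Enemy-tagged hits, while FireProjectile spawns a projectile with speed and damage.
; Ammo checks and OnShoot consumption switch on ammo type to use the player character's Bullet, Shell, Rocket or Cell pools.
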(event `self.ReceiveBeginPlay`
  (bind _asbp_first_person_character (cast `/Game/FirstPerson/Blueprints/BP_FirstPersonCharacter` (`GameplayStatics.GetPlayerCharacter` 0)))
  (set `self.PlayerCharacterRef` _asbp_first_person_character)
  (`self.UpdateDescription`))

(event `StartShooting`)

(event `StopShooting`)

(event `UpdateDescription`)

(event `OnShoot`
  (`self.DecreaseAmmoAmount`))

(fn `DecreaseAmmoAmount`
  (switch `/Game/Blueprints/Weapons/Ammo` (`self.AmmoType`)
    (:`NewEnumerator0`
      (`self.DecreaseBulletAmount`))
    (:`NewEnumerator1`
      (`self.DecreaseShellAmount`))
    (:`NewEnumerator2`
      (`self.DecreaseRocketAmount`))
    (:`NewEnumerator3`
      (`self.DecreaseCellAmount`))))

(fn `DecreaseBulletAmount`
  (set `/Game/FirstPerson/Blueprints/BP_FirstPersonCharacter.BulletAmount` (- (`/Game/FirstPerson/Blueprints/BP_FirstPersonCharacter.BulletAmount` (`self.PlayerCharacterRef`)) (`self.NeedAmmoToFire`)) (`self.PlayerCharacterRef`)))

(fn `DecreaseCellAmount`
  (set `/Game/FirstPerson/Blueprints/BP_FirstPersonCharacter.CellAmount` (- (`/Game/FirstPerson/Blueprints/BP_FirstPersonCharacter.CellAmount` (`self.PlayerCharacterRef`)) (`self.NeedAmmoToFire`)) (`self.PlayerCharacterRef`)))

(fn `DecreaseRocketAmount`
  (set `/Game/FirstPerson/Blueprints/BP_FirstPersonCharacter.RocketAmount` (- (`/Game/FirstPerson/Blueprints/BP_FirstPersonCharacter.RocketAmount` (`self.PlayerCharacterRef`)) (`self.NeedAmmoToFire`)) (`self.PlayerCharacterRef`)))

(fn `DecreaseShellAmount`
  (set `/Game/FirstPerson/Blueprints/BP_FirstPersonCharacter.ShellAmount` (- (`/Game/FirstPerson/Blueprints/BP_FirstPersonCharacter.ShellAmount` (`self.PlayerCharacterRef`)) (`self.NeedAmmoToFire`)) (`self.PlayerCharacterRef`)))

(fn `FireProjectile`
  (`|SpawnActorFromClass` (`self.ProjectileClass`) (`SceneComponent.K2_GetComponentToWorld` (`self.ProjectileTransform`)) "Undefined" "OverrideRootScale" null (`self.ProjectileSpeed`) (`self.WeaponDamage`) null))

(fn `FireWeapon`
  (bind _returnvalue (`SceneComponent.K2_GetComponentLocation` (`self.LineTrace`)))
  (bind (_returnvalue_roll _returnvalue_pitch _returnvalue_yaw) (`KismetMathLibrary.BreakRotator` (`KismetMathLibrary.FindLookAtRotation` (`self.K2_GetActorLocation` (`GameplayStatics.GetPlayerCharacter` 0)) (`self.K2_GetActorLocation`))))
  (bind (_outhit _returnvalue_2) (`KismetSystemLibrary.LineTraceSingleForObjects` _returnvalue (+ _returnvalue (* (`KismetMathLibrary.GetForwardVector` (`SceneComponent.K2_GetComponentRotation` (`self.LineTrace`))) (`self.LineTraceDistance`))) (`|MakeArray` "ObjectTypeQuery1" "ObjectTypeQuery2" "ObjectTypeQuery3" :!type "EObjectTypeQuery Enum") false (`|MakeArray` self (`GameplayStatics.GetPlayerCharacter` 0) :!type "Actor Object Reference") "ForDuration"))
  (if _returnvalue_2
    (bind (_bblockinghit _binitialoverlap _time _distance _location _impactpoint _normal _impactnormal _physmat _hitactor) (`GameplayStatics.BreakHitResult` _outhit))
    (`GameplayStatics.ApplyDamage` _hitactor (`self.WeaponDamage`))
    (if (`self.ActorHasTag` _hitactor "Enemy")
      (`|SpawnActorFromClass` "/Game/Enemies/BP_BloodEffect.BP_BloodEffect_C" (`KismetMathLibrary.MakeTransform` _location (`KismetMathLibrary.MakeRotator` 0.0 0.0 _returnvalue_yaw)) "Undefined" "OverrideRootScale" null null))))

(fn `HasEnoughAmmo?`
  (returns (HasAmmo :type Boolean))
  (switch `/Game/Blueprints/Weapons/Ammo` (`self.AmmoType`)
    (:`NewEnumerator0`
      (return (> (`/Game/FirstPerson/Blueprints/BP_FirstPersonCharacter.BulletAmount` (`self.PlayerCharacterRef`)) 0)))
    (:`NewEnumerator1`
      (return (> (`/Game/FirstPerson/Blueprints/BP_FirstPersonCharacter.ShellAmount` (`self.PlayerCharacterRef`)) 0)))
    (:`NewEnumerator2`
      (return (> (`/Game/FirstPerson/Blueprints/BP_FirstPersonCharacter.RocketAmount` (`self.PlayerCharacterRef`)) 0)))
    (:`NewEnumerator3`
      (return (> (`/Game/FirstPerson/Blueprints/BP_FirstPersonCharacter.CellAmount` (`self.PlayerCharacterRef`)) 0)))))

(fn `UserConstructionScript`)