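; BP_Shotgun is a shotgun weapon Blueprint that fires with Paper2D flipbook animation.
; StartShooting calls HasEnoughAmmo, then enters a DoOnce gate that runs OnShoot and FireWeapon and switches to the fire flipbook.
; A delay equal to that flipbook's length restores the idle flipbook and calls ResetFire to reopen the gate, so the animation sets the fire rate.
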(event `self.StartShooting`
  (`self.HasEnoughAmmo?`)
  (`/Engine/EditorBlueprintResources/StandardMacros.DoOnce` false :!label _label
    (:`Completed`
      (`self.OnShoot`)
      (`self.FireWeapon`)
      (`PaperFlipbookComponent.SetFlipbook` (`self.WeaponFlipbook`) "/Game/Sprites/Weapons/Shotgun/Sprites/PFB_Shotgun_Fire.PFB_Shotgun_Fire")
      (`KismetSystemLibrary.Delay` (`PaperFlipbookComponent.GetFlipbookLength` (`self.WeaponFlipbook`)))
      (`PaperFlipbookComponent.SetFlipbook` (`self.WeaponFlipbook`) "/Game/Sprites/Weapons/Shotgun/Sprites/PFB_Shotgun_Ide.PFB_Shotgun_Ide")
      (`self.ResetFire`))))

(event `ResetFire`
  (goto _label :!via `Reset`))

(fn `UserConstructionScript`
  (`parent.UserConstructionScript`))