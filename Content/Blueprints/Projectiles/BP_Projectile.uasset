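; Paper2D projectile actor that damages whatever it hits and then plays a destruction animation.
; The construction script sets both initial and max speed of its projectile movement from one speed variable.
; On hit it applies damage, rescales the flipbook and swaps it to the destroyed animation, then destroys itself after a delay equal to that flipbook's length.
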(event `self.ReceiveHit`
  (params (MyComp :type "PrimitiveComponent Object Reference") (Other :type "Actor Object Reference") (OtherComp :type "PrimitiveComponent Object Reference") (bSelfMoved :type Boolean) (HitLocation :type "Vector Structure") (HitNormal :type "Vector Structure") (NormalImpulse :type "Vector Structure") (Hit :type "HitResult Structure (by ref)"))
  (`GameplayStatics.ApplyDamage` Other (`self.ProjectileDamage`))
  (`SceneComponent.SetWorldScale3D` (`self.PaperFlipbook`) (`self.DestroyedScale`))
  (`PaperFlipbookComponent.SetFlipbook` (`self.PaperFlipbook`) (`self.DestroyedProjectile`))
  (`KismetSystemLibrary.Delay` (`PaperFlipbookComponent.GetFlipbookLength` (`self.PaperFlipbook`)))
  (`self.K2_DestroyActor`))

(fn `UserConstructionScript`
  (set `ProjectileMovementComponent.InitialSpeed` (`self.ProjectileSpeed`) (`self.ProjectileMovement`))
  (set `ProjectileMovementComponent.MaxSpeed` (`self.ProjectileSpeed`) (`self.ProjectileMovement`)))