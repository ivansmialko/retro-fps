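; BP_AmmoPickUp is a sprite-based ammo pickup that grants the player a set amount of one ammo type.
; The construction script picks a Paper2D flipbook to match the ammo type, and each tick the actor yaws toward the player as a billboard.
; On the first box overlap by the first-person character, it adds the ammo, refreshes the HUD count and destroys itself.
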(event `self.ReceiveTick`
  (params (DeltaSeconds :type "Float (single-precision)"))
  (bind (_returnvalue_roll _returnvalue_pitch _returnvalue_yaw) (`KismetMathLibrary.BreakRotator` (`KismetMathLibrary.FindLookAtRotation` (`self.K2_GetActorLocation`) (`self.K2_GetActorLocation` (`GameplayStatics.GetPlayerCharacter` 0)))))
  (`self.K2_SetActorRotation` (`KismetMathLibrary.MakeRotator` 0.0 0.0 _returnvalue_yaw)))

(event `self.Box.OnComponentBeginOverlap`
  (params (OverlappedComponent :type "PrimitiveComponent Object Reference") (OtherActor :type "Actor Object Reference") (OtherComp :type "PrimitiveComponent Object Reference") (OtherBodyIndex :type Integer) (bFromSweep :type Boolean) (SweepResult :type "HitResult Structure (by ref)"))
  (bind _asbp_first_person_character (cast `/Game/FirstPerson/Blueprints/BP_FirstPersonCharacter` OtherActor))
  (`/Engine/EditorBlueprintResources/StandardMacros.DoOnce` false
    (:`Completed`
      (`self.AddAmmoToPlayer` _asbp_first_person_character)
      (`self.K2_DestroyActor`))))

(fn `AddAmmoToPlayer`
  (params (Player :type "/Game/FirstPerson/Blueprints/BP_FirstPersonCharacter Object Reference"))
  (locals (LocalPlayer :type "/Game/FirstPerson/Blueprints/BP_FirstPersonCharacter Object Reference") (LocalPlayerHealth :type "Float (double-precision)" :default 0.0))
  (bind _output_get (set `local.LocalPlayer` Player))
  (`/Game/FirstPerson/Blueprints/BP_FirstPersonCharacter.AddAmmoAmountByType` _output_get (`self.AmmoType`) (`self.AmmoAmount`))
  (`/Game/Blueprints/UI/W_PlayerHUD.UpdateCurrentAmmoAmount` (`/Game/FirstPerson/Blueprints/BP_FirstPersonCharacter.PlayerHUD_Ref` (`local.LocalPlayer`)))
  (return))

(fn `UserConstructionScript`
  (switch `/Game/Blueprints/Weapons/Ammo` (`self.AmmoType`)
    (:`NewEnumerator0`
      (`PaperFlipbookComponent.SetFlipbook` (`self.PaperFlipbook`) "/Game/Sprites/Items/PFB_Item_Ammo_Bullet.PFB_Item_Ammo_Bullet"))
    (:`NewEnumerator1`
      (`PaperFlipbookComponent.SetFlipbook` (`self.PaperFlipbook`) "/Game/Sprites/Items/PFB_Item_Ammo_Shell.PFB_Item_Ammo_Shell"))
    (:`NewEnumerator2`
      (`PaperFlipbookComponent.SetFlipbook` (`self.PaperFlipbook`) "/Game/Sprites/Items/PFB_Item_Ammo_Rocket.PFB_Item_Ammo_Rocket"))
    (:`NewEnumerator3`
      (`PaperFlipbookComponent.SetFlipbook` (`self.PaperFlipbook`) "/Game/Sprites/Items/PFB_Item_Ammo_Cell.PFB_Item_Ammo_Cell"))))