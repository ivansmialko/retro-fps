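; BP_HealthPickUp is a health pickup that restores HealthAmount to the first-person player on touch.
; Each tick it yaws to face player 0, billboard style.
; When BP_FirstPersonCharacter overlaps its box, a DoOnce gate runs AddHealthToPlayer, which clamps the new health to MaxHealth and refreshes the player HUD, then the pickup destroys itself.
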(event `self.ReceiveTick`
  (params (DeltaSeconds :type "Float (single-precision)"))
  (bind (_returnvalue_roll _returnvalue_pitch _returnvalue_yaw) (`KismetMathLibrary.BreakRotator` (`KismetMathLibrary.FindLookAtRotation` (`self.K2_GetActorLocation`) (`self.K2_GetActorLocation` (`GameplayStatics.GetPlayerCharacter` 0)))))
  (`self.K2_SetActorRotation` (`KismetMathLibrary.MakeRotator` 0.0 0.0 _returnvalue_yaw)))

(event `self.Box.OnComponentBeginOverlap`
  (params (OverlappedComponent :type "PrimitiveComponent Object Reference") (OtherActor :type "Actor Object Reference") (OtherComp :type "PrimitiveComponent Object Reference") (OtherBodyIndex :type Integer) (bFromSweep :type Boolean) (SweepResult :type "HitResult Structure (by ref)"))
  (bind _asbp_first_person_character (cast `/Game/FirstPerson/Blueprints/BP_FirstPersonCharacter` OtherActor))
  (`/Engine/EditorBlueprintResources/StandardMacros.DoOnce` false
    (:`Completed`
      (`self.AddHealthToPlayer` _asbp_first_person_character)
      (`self.K2_DestroyActor`))))

(fn `AddHealthToPlayer`
  (params (Player :type "/Game/FirstPerson/Blueprints/BP_FirstPersonCharacter Object Reference"))
  (locals (LocalPlayer :type "/Game/FirstPerson/Blueprints/BP_FirstPersonCharacter Object Reference") (LocalPlayerHealth :type "Float (double-precision)" :default 0.0))
  (bind _output_get (set `local.LocalPlayer` Player))
  (set `local.LocalPlayerHealth` (`/Game/FirstPerson/Blueprints/BP_FirstPersonCharacter.Health` _output_get))
  (set `/Game/FirstPerson/Blueprints/BP_FirstPersonCharacter.Health` (`KismetMathLibrary.FClamp` (+ (`local.LocalPlayerHealth`) (`self.HealthAmount`)) 0.0 (`/Game/FirstPerson/Blueprints/BP_FirstPersonCharacter.MaxHealth` (`local.LocalPlayer`))) (`local.LocalPlayer`))
  (`/Game/Blueprints/UI/W_PlayerHUD.UpdatePlayerHealth` (`/Game/FirstPerson/Blueprints/BP_FirstPersonCharacter.PlayerHUD_Ref` (`local.LocalPlayer`)))
  (return))

(fn `UserConstructionScript`)