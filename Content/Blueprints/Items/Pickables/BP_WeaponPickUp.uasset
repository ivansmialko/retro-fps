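; Weapon pickup actor that shows a weapon's sprite and gives that weapon to the first-person player character.
; The construction script maps the WeaponType enum to a weapon class, then takes the Paper2D sprite from that class's defaults and applies WeaponScale.
; Every tick it yaws toward the player like a billboard.
; On sphere overlap it calls PickUpWeapon on the character and destroys itself.
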(event `self.ReceiveTick`
  (params (DeltaSeconds :type "Float (single-precision)"))
  (bind (_returnvalue_roll _returnvalue_pitch _returnvalue_yaw) (`KismetMathLibrary.BreakRotator` (`KismetMathLibrary.FindLookAtRotation` (`self.K2_GetActorLocation`) (`self.K2_GetActorLocation` (`GameplayStatics.GetPlayerCharacter` 0)))))
  (`self.K2_SetActorRotation` (`KismetMathLibrary.MakeRotator` 0.0 0.0 _returnvalue_yaw)))

(event `self.Sphere.OnComponentBeginOverlap`
  (params (OverlappedComponent :type "PrimitiveComponent Object Reference") (OtherActor :type "Actor Object Reference") (OtherComp :type "PrimitiveComponent Object Reference") (OtherBodyIndex :type Integer) (bFromSweep :type Boolean) (SweepResult :type "HitResult Structure (by ref)"))
  (bind _asbp_first_person_character (cast `/Game/FirstPerson/Blueprints/BP_FirstPersonCharacter` OtherActor))
  (`/Game/FirstPerson/Blueprints/BP_FirstPersonCharacter.PickUpWeapon` _asbp_first_person_character (`self.WeaponClass`))
  (`self.K2_DestroyActor`))

(fn `SetWeaponImage`
  (params (WeaponClass :type "/Game/Blueprints/Weapons/BP_BaseWeapon Class Reference"))
  (`PaperSpriteComponent.SetSprite` (`self.PaperSprite`) (`.WeaponImage` (defaults `Object` WeaponClass)))
  (`SceneComponent.SetWorldScale3D` (`self.PaperSprite`) (`self.WeaponScale`)))

(fn `UserConstructionScript`
  (switch `/Game/Blueprints/Weapons/Weapon` (`self.WeaponType`)
    (:`NewEnumerator0`
      (bind _output_get (set `self.WeaponClass` "/Game/Blueprints/Weapons/BP_Shotgun.BP_Shotgun_C"))
      (`self.SetWeaponImage` _output_get))
    (:`NewEnumerator1`
      (bind _output_get_2 (set `self.WeaponClass` "/Game/Blueprints/Weapons/BP_SubmachineGun.BP_SubmachineGun_C"))
      (`self.SetWeaponImage` _output_get_2))
    (:`NewEnumerator2`
      (bind _output_get_3 (set `self.WeaponClass` "/Game/Blueprints/Weapons/BP_PlasmaGun.BP_PlasmaGun_C"))
      (`self.SetWeaponImage` _output_get_3))
    (:`NewEnumerator3`
      (bind _output_get_4 (set `self.WeaponClass` "/Game/Blueprints/Weapons/BP_RPG.BP_RPG_C"))
      (`self.SetWeaponImage` _output_get_4))
    (:`NewEnumerator4`
      (bind _output_get_5 (set `self.WeaponClass` "/Game/Blueprints/Weapons/BP_BFG.BP_BFG_C"))
      (`self.SetWeaponImage` _output_get_5))
    (:`NewEnumerator5`
      (bind _output_get_6 (set `self.WeaponClass` "/Game/Blueprints/Weapons/BP_Chainsaw.BP_Chainsaw_C"))
      (`self.SetWeaponImage` _output_get_6))
    (:`NewEnumerator6`
      (bind _output_get_7 (set `self.WeaponClass` "/Game/Blueprints/Weapons/BP_Knife.BP_Knife_C"))
      (`self.SetWeaponImage` _output_get_7))))