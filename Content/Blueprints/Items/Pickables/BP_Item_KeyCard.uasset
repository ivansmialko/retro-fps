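; Key card pickup item, shown as a 2D Paper sprite whose red, orange or blue variant the construction script selects from CardType.
; Every tick it yaws along the line from the first player to itself, billboard style.
; Box overlap stores the first-person character reference.
; The logic that calls PickUpCardKey with the card type and destroys the actor is disconnected, so this graph never grants the card.
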(event `self.ReceiveTick`
  (params (DeltaSeconds :type "Float (single-precision)"))
  (bind (_returnvalue_roll _returnvalue_pitch _returnvalue_yaw) (`KismetMathLibrary.BreakRotator` (`KismetMathLibrary.FindLookAtRotation` (`self.K2_GetActorLocation` (`GameplayStatics.GetPlayerCharacter` 0)) (`self.K2_GetActorLocation`))))
  (`self.K2_SetActorRotation` (`KismetMathLibrary.MakeRotator` 0.0 0.0 _returnvalue_yaw)))

(event `self.Box.OnComponentBeginOverlap`
  (params (OverlappedComponent :type "PrimitiveComponent Object Reference") (OtherActor :type "Actor Object Reference") (OtherComp :type "PrimitiveComponent Object Reference") (OtherBodyIndex :type Integer) (bFromSweep :type Boolean) (SweepResult :type "HitResult Structure (by ref)"))
  (bind _asbp_first_person_character (cast `/Game/FirstPerson/Blueprints/BP_FirstPersonCharacter` OtherActor))
  (bind _output_get (set `self.PlayerCharacterRef` _asbp_first_person_character)))

(fn `UserConstructionScript`
  (switch `/Game/Blueprints/Items/KeyCard` (`self.CardType`)
    (:`NewEnumerator0`
      (`PaperSpriteComponent.SetSprite` (`self.PaperSprite`) "/Game/Sprites/Items/Sprites/SPR_Item_Key_Red.SPR_Item_Key_Red"))
    (:`NewEnumerator1`
      (`PaperSpriteComponent.SetSprite` (`self.PaperSprite`) "/Game/Sprites/Items/Sprites/SPR_Item_Key_Orange.SPR_Item_Key_Orange"))
    (:`NewEnumerator2`
      (`PaperSpriteComponent.SetSprite` (`self.PaperSprite`) "/Game/Sprites/Items/Sprites/SPR_Item_Key_Blue.SPR_Item_Key_Blue"))))