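; BP_Floating_Item is a decorative flipbook item that floats in the level and turns with the player's position.
; The construction script applies the configured flipbook and scale and stores the actor's start position.
; Each Tick sets yaw from the player-to-item look-at direction, billboard style, and calls Play on a timeline.
; The timeline lerps the location between the start position and that position plus MovementVector.
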(event `self.ReceiveTick`
  (params (DeltaSeconds :type "Float (single-precision)"))
  (bind (_returnvalue_roll _returnvalue_pitch _returnvalue_yaw) (`KismetMathLibrary.BreakRotator` (`KismetMathLibrary.FindLookAtRotation` (`self.K2_GetActorLocation` (`GameplayStatics.GetPlayerCharacter` 0)) (`self.K2_GetActorLocation`))))
  (`self.K2_SetActorRotation` (`KismetMathLibrary.MakeRotator` 0.0 0.0 _returnvalue_yaw))
  (bind (_direction _newtrack_0) (`Timeline|FloatingTimeline` :`NewTime` DeltaSeconds)
    (:`Update`
      (`self.K2_SetActorLocation` (`KismetMathLibrary.VLerp` (`self.StartPosition`) (+ (`self.StartPosition`) (`self.MovementVector`)) _newtrack_0)))))

(fn `UserConstructionScript`
  (`PaperFlipbookComponent.SetFlipbook` (`self.PaperFlipbook`) (`self.DecorationFlipbook`))
  (`SceneComponent.SetWorldScale3D` (`self.PaperFlipbook`) (`self.DecorationScale`))
  (set `self.StartPosition` (`self.K2_GetActorLocation`)))