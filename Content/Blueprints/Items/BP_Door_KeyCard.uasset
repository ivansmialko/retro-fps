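; Sliding door that opens only for a first-person character holding the keycard matching its KeyType.
; The construction script caches the cube's closed location, computes a target raised by SlideHeight, and colors the door red, orange or blue by key type.
; Entering the collision box with the card plays a Timeline that lerps the cube upward; leaving with the card reverses it.
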(event `self.CollisionBox.OnComponentBeginOverlap`
  (params (OverlappedComponent :type "PrimitiveComponent Object Reference") (OtherActor :type "Actor Object Reference") (OtherComp :type "PrimitiveComponent Object Reference") (OtherBodyIndex :type Integer) (bFromSweep :type Boolean) (SweepResult :type "HitResult Structure (by ref)"))
  (bind _asbp_first_person_character (cast `/Game/FirstPerson/Blueprints/BP_FirstPersonCharacter` OtherActor))
  (bind _havethiscard (`/Game/FirstPerson/Blueprints/BP_FirstPersonCharacter.HaveCardByType` _asbp_first_person_character (`self.KeyType`)))
  (if _havethiscard
    (bind (_direction _newtrack_0) (`Timeline|Timeline` :!label _label)
      (:`Update`
        (`SceneComponent.K2_SetWorldLocation` (`self.Cube`) (`KismetMathLibrary.VLerp` (`self.DefaultLocation`) (`self.TargetLocation`) _newtrack_0) false false)))))

(event `self.CollisionBox.OnComponentEndOverlap`
  (params (OverlappedComponent :type "PrimitiveComponent Object Reference") (OtherActor :type "Actor Object Reference") (OtherComp :type "PrimitiveComponent Object Reference") (OtherBodyIndex :type Integer))
  (bind _asbp_first_person_character (cast `/Game/FirstPerson/Blueprints/BP_FirstPersonCharacter` OtherActor))
  (bind _havethiscard (`/Game/FirstPerson/Blueprints/BP_FirstPersonCharacter.HaveCardByType` _asbp_first_person_character (`self.KeyType`)))
  (if _havethiscard
    (goto _label :!via `Reverse`)))

(fn `UserConstructionScript`
  (bind _output_get (set `self.DefaultLocation` (`SceneComponent.K2_GetComponentLocation` (`self.Cube`))))
  (set `self.TargetLocation` (`KismetMathLibrary.MakeVector` (.x _output_get) (.y _output_get) (+ (.z _output_get) (`self.SlideHeight`))))
  (switch `/Game/Blueprints/Items/KeyCard` (`self.KeyType`)
    (:`NewEnumerator0`
      (`PrimitiveComponent.SetMaterial` (`self.Cube`) 0 "/Game/Sprites/Items/M_RedDoor.M_RedDoor"))
    (:`NewEnumerator1`
      (`PrimitiveComponent.SetMaterial` (`self.Cube`) 0 "/Game/Sprites/Items/M_OrangeDoor.M_OrangeDoor"))
    (:`NewEnumerator2`
      (`PrimitiveComponent.SetMaterial` (`self.Cube`) 0 "/Game/Sprites/Items/M_BlueDoor.M_BlueDoor"))))