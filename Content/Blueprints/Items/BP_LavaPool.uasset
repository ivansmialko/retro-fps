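; BP_LavaPool is a hazard actor that repeatedly damages the first-person player character while it is inside its box trigger.
; Overlap begin stores the character and starts a looping timer at DamageFrequency that calls DamagePlayer to apply Damage.
; Overlap end by the character clears the timer.
; The first damage lands one interval after entry, as nothing applies it immediately on overlap.
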(event `self.Box.OnComponentBeginOverlap`
  (params (OverlappedComponent :type "PrimitiveComponent Object Reference") (OtherActor :type "Actor Object Reference") (OtherComp :type "PrimitiveComponent Object Reference") (OtherBodyIndex :type Integer) (bFromSweep :type Boolean) (SweepResult :type "HitResult Structure (by ref)"))
  (bind _asbp_first_person_character (cast `/Game/FirstPerson/Blueprints/BP_FirstPersonCharacter` OtherActor))
  (set `self.PlayerCharacterRef` _asbp_first_person_character)
  (bind _returnvalue (`KismetSystemLibrary.K2_SetTimerDelegate` (delegate `DamagePlayer`) (`self.DamageFrequency`) true))
  (set `self.LavaTimerHandle` _returnvalue))

(event `DamagePlayer`
  (`GameplayStatics.ApplyDamage` (`self.PlayerCharacterRef`) (`self.Damage`)))

(event `self.Box.OnComponentEndOverlap`
  (params (OverlappedComponent :type "PrimitiveComponent Object Reference") (OtherActor :type "Actor Object Reference") (OtherComp :type "PrimitiveComponent Object Reference") (OtherBodyIndex :type Integer))
  (cast `/Game/FirstPerson/Blueprints/BP_FirstPersonCharacter` OtherActor)
  (`KismetSystemLibrary.K2_ClearAndInvalidateTimerHandle` (`self.LavaTimerHandle`)))

(fn `UserConstructionScript`)